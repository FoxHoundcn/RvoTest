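; BP_RvoController drives an RVO agent simulation and keeps feeding it agents around its own location.
; On BeginPlay it initializes the RvoController and starts two looping timers, one ticking the simulation at its TickDeltaTime and one adding an agent every second.
; Each add tries to wake an existing agent at a random point on a surrounding ring, otherwise spawns and registers a new BP_RvoAgent, pooling-style.
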(event Custom|RvoTick
  (Class|RvoController|RVOTick (Variables|Default|GetRvoController)))

(event Custom|NewAgent
  (bind _returnvalue (Math|Random|RandomFloatinRange 0.0 3.6e+02))
  (bind _returnvalue_2 (Transformation|GetActorLocation))
  (bind _returnvalue_3 (Math|Vector|MakeVector 1e+03 0.0 0.0))
  (bind _returnvalue_4 (Math|Vector|RotateVectorAroundAxis _returnvalue_3 _returnvalue "0.000000,0.000000,1.000000"))
  (bind _returnvalue_5 (+ _returnvalue_2 _returnvalue_4))
  (bind _returnvalue_6 (Class|RvoController|RVOWakeUpAgent (Variables|Default|GetRvoController) _returnvalue_5))
  (Utilities|IsValid _returnvalue_6
    (:Is%20Not%20Valid
      (bind _returnvalue_7 (Game|SpawnActorfromClass "/Game/BP_RvoAgent.BP_RvoAgent_C" (Math|Transform|MakeTransform _returnvalue_5) "Undefined" "MultiplyWithRoot" 0 0))
      (bind _returnvalue_8 (Class|RvoController|RVOHostingActor (Variables|Default|GetRvoController) _returnvalue_7))
      (if _returnvalue_8
        (Development|PrintString "New Agent")))))

(event EventBeginPlay
  (bind _rvocontroller (Variables|Default|GetRvoController))
  (Class|RvoController|RVOInit _rvocontroller)
  (Utilities|Time|SetTimerbyEvent (delegate Custom|RvoTick) (Variables|/Script/Rvo2D.RvoController|GetTickDeltaTime _rvocontroller) true)
  (Utilities|Time|SetTimerbyEvent (delegate Custom|NewAgent) 1.0 true))

(event Collision|EventActorBeginOverlap
  (params (OtherActor :type Actor%20Object%20Reference)))

(event EventTick
  (params (DeltaSeconds :type Float%20%28single-precision%29)))

(fn ConstructionScript)